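; HUD for the Dungeon Master companion that creates the main canvas on BeginPlay and manages NPC and village widgets on it.
; NPC widgets are tracked in a widget-to-data map, so creation expands an existing collapsed widget or adds a new one, and removal clears it.
; Lookup matches character sheet names but returns after the first map entry.
; AddVillageOverlay adds the village overlay to the canvas and announces it.
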(event `self.ReceiveBeginPlay`
  (bind _returnvalue (`|CreateWidget` "/Game/DungeonMasterCompanion/Blueprints/Core/WBP_MainCanvas.WBP_MainCanvas_C"))
  (bind _output_get (set `self.MainCanvas` _returnvalue))
  (`self.OnMainCanvasCreated` self _output_get)
  (`UserWidget.AddToViewport` _output_get 0))

(event `/Game/DungeonMasterCompanion/Blueprints/Core/BPI_CharacterWidgets.CreateNpcWidget`
  (params (NpcData :type "NpcData Structure"))
  (bind _output (`self.GetNpcWidget` NpcData))
  (`/Engine/EditorBlueprintResources/StandardMacros.IsValid` _output
    (:`Is Valid`
      (if (not (`/Game/DungeonMasterCompanion/Blueprints/UserInterface/WBP_NPC.GetIsExpanded` _output))
        (`/Game/DungeonMasterCompanion/Blueprints/UserInterface/WBP_NPC.SetExpanded` _output true)))
    (:`Is Not Valid`
      (bind _returnvalue (`|CreateWidget` "/Game/DungeonMasterCompanion/Blueprints/UserInterface/WBP_NPC.WBP_NPC_C" null NpcData))
      (`/Game/DungeonMasterCompanion/Blueprints/Core/WBP_MainCanvas.AddToMainCanvas` (`self.MainCanvas`) _returnvalue)
      (`BlueprintMapLibrary.Map_Add` (`self.NpcWidgetOnScreen`) _returnvalue NpcData))))

(event `/Game/DungeonMasterCompanion/Blueprints/Core/BPI_CharacterWidgets.RemoveNpcWidget`
  (params (NpcData :type "NpcData Structure"))
  (bind _output (`self.GetNpcWidget` NpcData))
  (`/Engine/EditorBlueprintResources/StandardMacros.IsValid` _output
    (:`Is Valid`
      (bind _returnvalue (`BlueprintMapLibrary.Map_Remove` (`self.NpcWidgetOnScreen`) _output))
      (if _returnvalue
        (`Widget.RemoveFromParent` _output)))))

(fn `AddVillageOverlay`
  (bind _returnvalue (`|CreateWidget` "/Game/DungeonMasterCompanion/Blueprints/VillageManager/UserInterface/WBP_VillageOverlay.WBP_VillageOverlay_C"))
  (set `self.VillageOverlay` _returnvalue)
  (`PanelWidget.AddChild` (`MainCanvas.MainOverlay` (`self.MainCanvas`)) _returnvalue)
  (`/Game/DungeonMasterCompanion/Blueprints/FunctionLibraries/BPFL_UserInterface.SetAlignmentAndPadding` (`self.VillageOverlay`))
  (`self.OnVillageOverlayAdded` (`self.VillageOverlay`)))

(fn `GetNpcWidget`
  (params (NpcData :type "NpcData Structure"))
  (returns (Output :type "/Game/DungeonMasterCompanion/Blueprints/UserInterface/WBP_NPC Object Reference"))
  (bind _values (`BlueprintMapLibrary.Map_Values` (`self.NpcWidgetOnScreen`)))
  (for (_array_element _array_index) _values
    (if (`KismetStringLibrary.EqualEqual_StrStr` (`.Name` (break `CharacterSheet` (`.CharacterSheet` (break `NpcData` _array_element)))) (`.Name` (break `CharacterSheet` (`.CharacterSheet` (break `NpcData` NpcData)))))
      (bind _keys (`BlueprintMapLibrary.Map_Keys` (`self.NpcWidgetOnScreen`)))
      (return (`|GetArrayItem` _keys _array_index))
      (else
        (return null))))
  (return null))

(fn `UserConstructionScript`)