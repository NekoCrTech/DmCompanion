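; BP_VillageManager handles building hover and selection in a village and drives the village overlay UI.
; On BeginPlay it binds to every BP_Building and to HUD creation events, through which it adds and initializes the overlay, and adds its Enhanced Input mapping.
; Hovering outlines a building and shows its data, clicking outlines it green and opens its panel.
; The deselect input closes the panel and clears the outline.
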(event `self.ReceiveBeginPlay`
  (`self.BindEvents`)
  (`self.AddInput`))

(event `OnBuildingClicked`
  (params (BuildingActor :type "BuildingActor Object Reference"))
  (bind _village_overlay (`self.Village Overlay`))
  (`self.SetSelectedBuildingOutline` BuildingActor)
  (`self.UpdateSelectedBuilding` BuildingActor)
  (`/Engine/EditorBlueprintResources/StandardMacros.IsValid` _village_overlay
    (:`Is Valid`
      (`/Game/DungeonMasterCompanion/Blueprints/VillageManager/UserInterface/WBP_VillageOverlay.OpenBuilding` _village_overlay true (`BuildingActor.BuildingData` (`self.SelectedBuilding`)))
      (set `BuildingActor.bIsSelected` true (`self.SelectedBuilding`)))))

(event `EnhancedInput|/Game/DungeonMasterCompanion/Blueprints/VillageManager/Input/IA_Deselect`
  (params (ActionValue :type Boolean) (ElapsedSeconds :type "Float (double-precision)") (TriggeredSeconds :type "Float (double-precision)") (InputAction :type "InputAction Object Reference" :default "/Game/DungeonMasterCompanion/Blueprints/VillageManager/Input/IA_Deselect.IA_Deselect"))
  (bind _selectedbuilding (`self.SelectedBuilding`))
  (:`Started`
    (bind _village_overlay (`self.Village Overlay`)
      (:`then`
        (`/Game/DungeonMasterCompanion/Blueprints/VillageManager/UserInterface/WBP_VillageOverlay.OpenBuilding` :`self` _village_overlay)
        (`/Game/DungeonMasterCompanion/Blueprints/FunctionLibraries/BPFL_Material.SetOutlineEnable` false (`BuildingActor.MeshComponent` _selectedbuilding))
        (set `BuildingActor.bIsSelected` false _selectedbuilding))
      (:`else`))))

(fn `AddInput`
  (bind _returnvalue (`GameplayStatics.GetPlayerController` 0))
  (`self.EnableInput` _returnvalue)
  (bind _asdmc_player_controller (cast `DMC_PlayerController` _returnvalue)
    (:`then`
      (`EnhancedInputSubsystemInterface.AddMappingContext` (pcsubsystem `EnhancedInputLocalPlayerSubsystem` _asdmc_player_controller) "/Game/DungeonMasterCompanion/Blueprints/VillageManager/Input/IMC_VillageManager.IMC_VillageManager" 0 (struct)))
    (:`CastFailed`
      (`KismetSystemLibrary.PrintString` "ERROR - Player Controller Not Found (Village Manager)" true true (struct :`R` 1.0 :`B` 0.019646 :`A` 1.0)))))

(fn `BindEvents`
  (bind _ashud_dmcompanion (cast `/Game/DungeonMasterCompanion/Blueprints/Core/HUD_DMCompanion` (`PlayerController.GetHUD` (`GameplayStatics.GetPlayerController` 0)) :!pure true))
  (add `/Game/DungeonMasterCompanion/Blueprints/Core/HUD_DMCompanion.OnMainCanvasCreated` _ashud_dmcompanion (`|CreateDelegate` :!event `OnMainCanvasCreated`))
  (add `/Game/DungeonMasterCompanion/Blueprints/Core/HUD_DMCompanion.OnVillageOverlayAdded` _ashud_dmcompanion (`|CreateDelegate` :!event `OnVillageOverlayCreated`))
  (bind _outactors (`GameplayStatics.GetAllActorsOfClass` "/Game/DungeonMasterCompanion/Blueprints/VillageManager/Building/BP_Building.BP_Building_C"))
  (bind _output_get (set `self.Buildings` _outactors))
  (for _array_element _output_get
    (add `BuildingActor.OnBuildingClicked` _array_element (`|CreateDelegate` :!event `OnBuildingClicked`))
    (add `BuildingActor.OnBuildingHovered` _array_element (`|CreateDelegate` :!event `OnBuildingHovered`))))

(fn `OnBuildingHovered`
  (params (BuildingActor :type "BuildingActor Object Reference"))
  (bind _hoveredbuilding (`self.HoveredBuilding`))
  (`/Engine/EditorBlueprintResources/StandardMacros.IsValid` BuildingActor
    (:`Is Valid`
      (bind _output_get (set `self.HoveredBuilding` (`local.BuildingActor`)))
      (`/Game/DungeonMasterCompanion/Blueprints/FunctionLibraries/BPFL_Material.SetOutlineEnable` true (`BuildingActor.MeshComponent` _output_get) (struct :`R` 1.0 :`G` 0.827258 :`A` 1.0) 3.0)
      (`self.UpdateHoveredBuilding` _hoveredbuilding)
      (`VillageOverlay.SetBuilding` (`self.Village Overlay`) (`BuildingActor.BuildingData` _hoveredbuilding)))
    (:`Is Not Valid`
      (`/Game/DungeonMasterCompanion/Blueprints/FunctionLibraries/BPFL_Material.SetOutlineEnable` false (`BuildingActor.MeshComponent` (`self.HoveredBuilding`)))
      (set `self.HoveredBuilding` null)
      (`self.UpdateHoveredBuilding` null)
      (`VillageOverlay.HideBuildingName` (`self.Village Overlay`))
      (bind _selectedbuilding (`self.SelectedBuilding`)
        (:`then`
          (`/Game/DungeonMasterCompanion/Blueprints/FunctionLibraries/BPFL_Material.SetOutlineEnable` true (`BuildingActor.MeshComponent` _selectedbuilding) (struct :`G` 1.0 :`B` 0.174767 :`A` 1.0) 3.0))
        (:`else`)))))

(fn `OnMainCanvasCreated`
  (params (HUD :type "/Game/DungeonMasterCompanion/Blueprints/Core/HUD_DMCompanion Object Reference") (MainCanvas :type "/Game/DungeonMasterCompanion/Blueprints/Core/WBP_MainCanvas Object Reference"))
  (`/Game/DungeonMasterCompanion/Blueprints/Core/HUD_DMCompanion.AddVillageOverlay` HUD))

(fn `OnVillageOverlayCreated`
  (params (VillageOverlay :type "/Game/DungeonMasterCompanion/Blueprints/VillageManager/UserInterface/WBP_VillageOverlay Object Reference"))
  (bind _output_get (set `self.Village Overlay` VillageOverlay))
  (`VillageOverlay.SetVillage` _output_get (`self.Village`) self))

(fn `SetSelectedBuildingOutline`
  (params (NewBuilding :type "BuildingActor Object Reference"))
  (if (!= (`self.SelectedBuilding`) NewBuilding)
    (`/Game/DungeonMasterCompanion/Blueprints/FunctionLibraries/BPFL_Material.SetOutlineEnable` true (`BuildingActor.MeshComponent` (`local.NewBuilding`)) (struct :`G` 1.0 :`B` 0.391186 :`A` 1.0) 3.0)
    (bind _selectedbuilding (`self.SelectedBuilding`)
      (:`then`
        (`/Game/DungeonMasterCompanion/Blueprints/FunctionLibraries/BPFL_Material.SetOutlineEnable` false (`BuildingActor.MeshComponent` _selectedbuilding) (struct :`G` 1.0 :`B` 0.391186 :`A` 1.0) 3.0))
      (:`else`))))

(fn `UserConstructionScript`)