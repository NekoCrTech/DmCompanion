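; BPFL_Utilities is a utility function library with one function, MakeStringFromArray, which joins an array of strings into a single string.
; It loops over the array, prepending each element to the accumulated string and adding the separator between neighbours.
; Because each piece goes in front, the returned string lists the elements in reverse array order.
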(fn `MakeStringFromArray`
  (params (Array :type "Array of String") (SeperationString :type String :default ", "))
  (returns (ReturnValue :type String))
  (locals (String :type String))
  (for (_array_element _array_index) Array
    (set `local.String` (`KismetStringLibrary.Concat_StrStr` _array_element (`local.String`)))
    (if (!= _array_index (`KismetArrayLibrary.Array_LastIndex` (`local.Array`)))
      (set `local.String` (`KismetStringLibrary.Concat_StrStr` (`local.SeperationString`) (`local.String`)))))
  (return (`local.String`)))