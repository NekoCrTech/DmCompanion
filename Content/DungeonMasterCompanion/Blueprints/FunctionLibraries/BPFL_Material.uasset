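; Blueprint function library for material helpers in DungeonMasterCompanion, currently providing a toggle for outlines on static mesh components.
; SetOutlineEnable creates a new dynamic instance of MI_OutlineOverlay, sets its color, thickness and emissive multiplier, and assigns it as the component's overlay material.
; Disabling clears the overlay slot, so the outline never touches the mesh's base materials.
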(fn `SetOutlineEnable`
  (params (bIsEnabled :type Boolean) (StaticMeshComponent :type "StaticMeshComponent Object Reference") (Color :type "LinearColor Structure" :default (struct :`R` 1.0 :`G` 0.827258 :`A` 1.0)) (Thickness :type "Float (double-precision)" :default 1.0) (EmissiveMultiplier :type "Float (double-precision)" :default 1.0))
  (locals (MaterialDynamicInstance :type "MaterialInstanceDynamic Object Reference"))
  (if bIsEnabled
    (bind _returnvalue (`KismetMaterialLibrary.CreateDynamicMaterialInstance` null "/Game/DungeonMasterCompanion/Assets/Material/MI_OutlineOverlay.MI_OutlineOverlay"))
    (bind _output_get (set `local.MaterialDynamicInstance` _returnvalue))
    (`MaterialInstanceDynamic.SetVectorParameterValue` _output_get "Color" (`local.Color`))
    (`MaterialInstanceDynamic.SetScalarParameterValue` (`local.MaterialDynamicInstance`) "EmissiveMultiplier" (`local.EmissiveMultiplier`))
    (`MaterialInstanceDynamic.SetScalarParameterValue` (`local.MaterialDynamicInstance`) "OutlineThickness" (`local.Thickness`))
    (`MeshComponent.SetOverlayMaterial` (`local.StaticMeshComponent`) (`local.MaterialDynamicInstance`))
    (else
      (`MeshComponent.SetOverlayMaterial` (`local.StaticMeshComponent`) null))))