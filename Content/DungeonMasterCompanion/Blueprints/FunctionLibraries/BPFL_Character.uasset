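; Blueprint function library for the Dungeon Master Companion that derives character stats from a map of classes to levels.
; GetCombinedLevel sums every class level in the map, supporting multiclassed characters.
; GetProfBonus feeds that total through tiered level thresholds to return the D&D-style proficiency bonus.
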(fn `GetCombinedLevel`
  (params (ClassWithLevel :type "Map of ECharacterClass Enum to Integer"))
  (returns (ReturnValue :type Integer))
  (locals (CombinedLevel :type Integer))
  (bind _values (`BlueprintMapLibrary.Map_Values` ClassWithLevel))
  (for _array_element _values
    (set `local.CombinedLevel` (+ _array_element (`local.CombinedLevel`))))
  (return (`local.CombinedLevel`)))

(fn `GetProfBonus`
  (params (ClassWithLevel :type "Map of ECharacterClass Enum to Integer"))
  (returns (ReturnValue :type Integer))
  (locals (CombinedLevel :type Integer :default 0))
  (set `local.CombinedLevel` (`self.GetCombinedLevel` ClassWithLevel))
  (if (>= (`local.CombinedLevel`) 17)
    (return 6)
    (elif (>= (`local.CombinedLevel`) 13)
      (return 5)
      (elif (>= (`local.CombinedLevel`) 9)
        (return 4)
        (elif (>= (`local.CombinedLevel`) 5)
          (return 3)
          (else
            (return 2)))))))