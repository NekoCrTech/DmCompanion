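; Blueprint function library that calculates skill modifiers for a Dungeon Master companion app.
; GetSkillModifier sums the linked attribute's modifier, all skill bonuses and, if proficient, the proficiency bonus.
; GetLinkedAttributeModifier finds the attribute in DT_SkillDescription by the skill's enum name, returning -99 for unknown skills.
; If lookup fails, AnimalHandling and SleightOfHand both fall back to the "AnimalHandling" row, so SleightOfHand receives that row's attribute.
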(fn `GetLinkedAttributeModifier`
  (params (Skill :type "Skill Structure (by ref)") (Attributes :type "Attributes Structure (by ref)"))
  (returns (ReturnValue :type Integer) (Attribute :type "EAttribute Enum"))
  (locals (LinkedAttributeScore :type "AttributeScore Structure") (LinkedAttribute :type "EAttribute Enum"))
  (bind ((`SkillName` _skillname)) (break `Skill` Skill))
  (bind _linkedattributescore (`local.LinkedAttributeScore`))
  (bind (_strength _dexterity _constitution _intelligence _wisdom _charisma) (break `Attributes` (`local.Attributes`)))
  (bind _returnvalue (`|GetDataTableRow` "/Game/DungeonMasterCompanion/Blueprints/Data/DT_SkillDescription.DT_SkillDescription" (`KismetStringLibrary.Conv_StringToName` (`|GetEnumeratorNameAsString` _skillname)))
    (:`then`
      (set `local.LinkedAttribute` (`.LinkedAttribute` (break `SkillDescription` _returnvalue))))
    (:`RowNotFound`
      (if (`|EnumEquality` _skillname "AnimalHandling")
        (bind _returnvalue_2 (`|GetDataTableRow` "/Game/DungeonMasterCompanion/Blueprints/Data/DT_SkillDescription.DT_SkillDescription" "AnimalHandling")
          (:`then`
            (set `local.LinkedAttribute` (`.LinkedAttribute` (break `SkillDescription` _returnvalue_2)))))
        (elif (`|EnumEquality` _skillname "SleightOfHand")
          (bind _returnvalue_3 (`|GetDataTableRow` "/Game/DungeonMasterCompanion/Blueprints/Data/DT_SkillDescription.DT_SkillDescription" "AnimalHandling")
            (:`then`
              (set `local.LinkedAttribute` (`.LinkedAttribute` (break `SkillDescription` _returnvalue_3)))))
          (else
            (return -99 "Strength"))))))
  (switch `EAttribute` (`local.LinkedAttribute`)
    (:`Strength`
      (set `local.LinkedAttributeScore` _strength))
    (:`Dexterity`
      (set `local.LinkedAttributeScore` _dexterity))
    (:`Constitution`
      (set `local.LinkedAttributeScore` _constitution))
    (:`Intelligence`
      (set `local.LinkedAttributeScore` _intelligence))
    (:`Wisdom`
      (set `local.LinkedAttributeScore` _wisdom))
    (:`Charisma`
      (set `local.LinkedAttributeScore` _charisma)))
  (return (`/Game/DungeonMasterCompanion/Blueprints/FunctionLibraries/BPFL_Attributes.GetAttributeModifier` _linkedattributescore) (`.AttributeType` (break `AttributeScore` _linkedattributescore))))

(fn `GetSkillModifier`
  (params (Skill :type "Skill Structure") (Attributes :type "Attributes Structure") (ProficiencyBonus :type Integer))
  (returns (ReturnValue :type Integer) (Attribute :type "EAttribute Enum"))
  (locals (LinkedAttributeModifier :type Integer :default 0))
  (bind (_returnvalue _attribute) (`self.GetLinkedAttributeModifier` Skill Attributes))
  (set `local.LinkedAttributeModifier` _returnvalue)
  (bind _values (`BlueprintMapLibrary.Map_Values` (`.SkillBonuses` (break `Skill` (`local.Skill`)))))
  (for _array_element _values
    (set `local.LinkedAttributeModifier` (+ (`local.LinkedAttributeModifier`) _array_element)))
  (if (`.bIsProficient` (break `Skill` (`local.Skill`)))
    (set `local.LinkedAttributeModifier` (+ (`local.LinkedAttributeModifier`) (`local.ProficiencyBonus`))))
  (return (`local.LinkedAttributeModifier`) _attribute))