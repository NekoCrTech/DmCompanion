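; Function library of monster stat block math for the Dungeon Master companion, covering hit points and Challenge Rating lookups.
; Average HP and its dice formula derive from a size-based hit die, hit dice count and Constitution modifier, using half the die size per die.
; CR maps to proficiency bonus by range, to display text with low fractions, and to XP by near-equal matches, with no explicit fallback.
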(fn `GetAvgHpAndFormula`
  (params (Size :type "ESize Enum" :default "Tiny") (Constitution :type "AttributeScore Structure") (HitDiceCount :type Integer))
  (returns (AvgHp :type Integer) (Formula :type Text))
  (locals (SizeVar :type Integer))
  (switch `ESize` (`local.Size`)
    (:`Tiny`
      (set `local.SizeVar` 4))
    (:`Small`
      (set `local.SizeVar` 6))
    (:`Medium`
      (set `local.SizeVar` 8))
    (:`Large`
      (set `local.SizeVar` 10))
    (:`Huge`
      (set `local.SizeVar` 12))
    (:`Gargantuan`
      (set `local.SizeVar` 20)))
  (return (+ (* (/ (`local.SizeVar`) 2) (`local.HitDiceCount`)) (* (`/Game/DungeonMasterCompanion/Blueprints/FunctionLibraries/BPFL_Attributes.GetAttributeModifier` (`local.Constitution`)) (`local.HitDiceCount`))) (`|FormatText` "({HitDiceCount}d{SizeVar}+{MultipliedMod})" (`local.HitDiceCount`) (`local.SizeVar`) (* (`/Game/DungeonMasterCompanion/Blueprints/FunctionLibraries/BPFL_Attributes.GetAttributeModifier` (`local.Constitution`)) (`local.HitDiceCount`)))))

(fn `GetCrText`
  (params (CR :type "Float (double-precision)"))
  (returns (ReturnValue :type Text))
  (if (`KismetMathLibrary.NearlyEqual_FloatFloat` CR)
    (return "0")
    (elif (`KismetMathLibrary.NearlyEqual_FloatFloat` (`local.CR`) 0.125)
      (return "1/8")
      (elif (`KismetMathLibrary.NearlyEqual_FloatFloat` (`local.CR`) 0.25)
        (return "1/4")
        (elif (`KismetMathLibrary.NearlyEqual_FloatFloat` (`local.CR`) 0.5)
          (return "1/2")
          (else
            (return (`KismetTextLibrary.Conv_DoubleToText` (`local.CR`) "ToZero" false false 1 324 0 0))))))))

(fn `GetProfBonusFromCr`
  (params (CR :type "Float (double-precision)"))
  (returns (ReturnValue :type Integer))
  (if (`KismetMathLibrary.InRange_FloatFloat` CR 0.0 3.0)
    (return 2)
    (elif (`KismetMathLibrary.InRange_FloatFloat` (`local.CR`) 3.0 7.0 false)
      (return 3)
      (elif (`KismetMathLibrary.InRange_FloatFloat` (`local.CR`) 7.0 13.0 false)
        (return 4)
        (elif (`KismetMathLibrary.InRange_FloatFloat` (`local.CR`) 13.0 20.0 false)
          (return 5)
          (elif (`KismetMathLibrary.InRange_FloatFloat` (`local.CR`) 20.0 24.0 false)
            (return 6)
            (elif (`KismetMathLibrary.InRange_FloatFloat` (`local.CR`) 24.0 30.0 false)
              (return 7)
              (else
                (return 8)))))))))

(fn `GetXpFromCr`
  (params (CR :type "Float (double-precision)"))
  (returns (ReturnValue :type Integer))
  (if (`KismetMathLibrary.NearlyEqual_FloatFloat` (`local.CR`))
    (return 10)
    (elif (`KismetMathLibrary.NearlyEqual_FloatFloat` (`local.CR`) 0.125)
      (return 25)
      (elif (`KismetMathLibrary.NearlyEqual_FloatFloat` (`local.CR`) 0.25)
        (return 50)
        (elif (`KismetMathLibrary.NearlyEqual_FloatFloat` (`local.CR`) 0.5)
          (return 100)
          (elif (`KismetMathLibrary.NearlyEqual_FloatFloat` (`local.CR`) 1.0)
            (return 200)
            (elif (`KismetMathLibrary.NearlyEqual_FloatFloat` (`local.CR`) 2.0)
              (return 450)
              (elif (`KismetMathLibrary.NearlyEqual_FloatFloat` (`local.CR`) 3.0)
                (return 700)
                (elif (`KismetMathLibrary.NearlyEqual_FloatFloat` (`local.CR`) 4.0)
                  (return 1100)
                  (elif (`KismetMathLibrary.NearlyEqual_FloatFloat` (`local.CR`) 5.0)
                    (return 1800)
                    (elif (`KismetMathLibrary.NearlyEqual_FloatFloat` (`local.CR`) 6.0)
                      (return 2300)
                      (elif (`KismetMathLibrary.NearlyEqual_FloatFloat` (`local.CR`) 7.0)
                        (return 2900)
                        (elif (`KismetMathLibrary.NearlyEqual_FloatFloat` (`local.CR`) 8.0)
                          (return 3900)
                          (elif (`KismetMathLibrary.NearlyEqual_FloatFloat` (`local.CR`) 9.0)
                            (return 5000)
                            (elif (`KismetMathLibrary.NearlyEqual_FloatFloat` (`local.CR`) 10.0)
                              (return 5900)
                              (elif (`KismetMathLibrary.NearlyEqual_FloatFloat` (`local.CR`) 11.0)
                                (return 7200)
                                (elif (`KismetMathLibrary.NearlyEqual_FloatFloat` (`local.CR`) 12.0)
                                  (return 8400)
                                  (elif (`KismetMathLibrary.NearlyEqual_FloatFloat` (`local.CR`) 13.0)
                                    (return 10000)
                                    (elif (`KismetMathLibrary.NearlyEqual_FloatFloat` (`local.CR`) 14.0)
                                      (return 11500)
                                      (elif (`KismetMathLibrary.NearlyEqual_FloatFloat` (`local.CR`) 15.0)
                                        (return 13000)
                                        (elif (`KismetMathLibrary.NearlyEqual_FloatFloat` (`local.CR`) 16.0)
                                          (return 15000)
                                          (elif (`KismetMathLibrary.NearlyEqual_FloatFloat` (`local.CR`) 17.0)
                                            (return 18000)
                                            (elif (`KismetMathLibrary.NearlyEqual_FloatFloat` (`local.CR`) 18.0)
                                              (return 20000)
                                              (elif (`KismetMathLibrary.NearlyEqual_FloatFloat` (`local.CR`) 19.0)
                                                (return 22000)
                                                (elif (`KismetMathLibrary.NearlyEqual_FloatFloat` (`local.CR`) 20.0)
                                                  (return 25000)
                                                  (elif (`KismetMathLibrary.NearlyEqual_FloatFloat` (`local.CR`) 21.0)
                                                    (return 33000)
                                                    (elif (`KismetMathLibrary.NearlyEqual_FloatFloat` (`local.CR`) 22.0)
                                                      (return 41000)
                                                      (elif (`KismetMathLibrary.NearlyEqual_FloatFloat` (`local.CR`) 23.0)
                                                        (return 50000)
                                                        (elif (`KismetMathLibrary.NearlyEqual_FloatFloat` (`local.CR`) 24.0)
                                                          (return 62000)
                                                          (elif (`KismetMathLibrary.NearlyEqual_FloatFloat` (`local.CR`) 25.0)
                                                            (return 75000)
                                                            (elif (`KismetMathLibrary.NearlyEqual_FloatFloat` (`local.CR`) 26.0)
                                                              (return 90000)
                                                              (elif (`KismetMathLibrary.NearlyEqual_FloatFloat` (`local.CR`) 27.0)
                                                                (return 105000)
                                                                (elif (`KismetMathLibrary.NearlyEqual_FloatFloat` (`local.CR`) 28.0)
                                                                  (return 120000)
                                                                  (elif (`KismetMathLibrary.NearlyEqual_FloatFloat` (`local.CR`) 29.0)
                                                                    (return 135000)
                                                                    (elif (`KismetMathLibrary.NearlyEqual_FloatFloat` (`local.CR`) 30.0)
                                                                      (return 155000))))))))))))))))))))))))))))))))))))