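; Blueprint function library of ability score helpers for the Dungeon Master Companion, covering the six D&D-style attributes.
; Totals are the base value plus every value in the bonus map, and the modifier derives from that total as (total - 10) / 2.
; Lookups convert an attribute to its three-letter abbreviation and map a saving throw gameplay tag to its attribute via exact-match checks.
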(fn `GetAbbreviation`
  (params (Attribute :type "EAttribute Enum" :default "Strength"))
  (returns (ReturnValue :type Text))
  (switch `EAttribute` Attribute
    (:`Strength`
      (return "STR"))
    (:`Dexterity`
      (return "DEX"))
    (:`Constitution`
      (return "CON"))
    (:`Intelligence`
      (return "INT"))
    (:`Wisdom`
      (return "WIS"))
    (:`Charisma`
      (return "CHA"))))

(fn `GetAttributeModifier`
  (params (AttributeData :type "AttributeScore Structure"))
  (returns (ReturnValue :type Integer))
  (return (/ (- (`self.GetTotalAttribute` AttributeData) 10) 2)))

(fn `GetProfAttribute`
  (params (SavingThrow :type "GameplayTag Structure"))
  (returns (ReturnValue :type String))
  (if (`BlueprintGameplayTagLibrary.MatchesTag` SavingThrow (struct :`TagName` "SavingThrow.Charisma") true)
    (return "Charisma")
    (elif (`BlueprintGameplayTagLibrary.MatchesTag` (`local.SavingThrow`) (struct :`TagName` "SavingThrow.Constitution") true)
      (return "Constitution")
      (elif (`BlueprintGameplayTagLibrary.MatchesTag` (`local.SavingThrow`) (struct :`TagName` "SavingThrow.Dexterity") true)
        (return "Dexterity")
        (elif (`BlueprintGameplayTagLibrary.MatchesTag` (`local.SavingThrow`) (struct :`TagName` "SavingThrow.Intelligence") true)
          (return "Intelligence")
          (elif (`BlueprintGameplayTagLibrary.MatchesTag` (`local.SavingThrow`) (struct :`TagName` "SavingThrow.Strength") true)
            (return "Strength")
            (elif (`BlueprintGameplayTagLibrary.MatchesTag` (`local.SavingThrow`) (struct :`TagName` "SavingThrow.Wisdom") true)
              (return "Wisdom"))))))))

(fn `GetTotalAttribute`
  (params (AttributeData :type "AttributeScore Structure"))
  (returns (ReturnValue :type Integer))
  (locals (TempSum :type Integer))
  (bind (_attributetype _basevalue _attributebonuses) (break `AttributeScore` (`local.AttributeData`)))
  (set `local.TempSum` _basevalue)
  (if (`BlueprintMapLibrary.Map_IsNotEmpty` _attributebonuses)
    (bind _values (`BlueprintMapLibrary.Map_Values` _attributebonuses))
    (for _array_element _values
      (set `local.TempSum` (+ (`local.TempSum`) _array_element))))
  (return (`local.TempSum`)))